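; BP_TPSPlayer is a third-person shooter player Blueprint whose event graph logic is entirely disconnected, leaving every event empty.
; The unwired nodes cover camera-relative movement, look, jumping, crosshair UI, grenade/sniper gun switching and FOV zoom with a scope widget.
; Orphaned firing nodes spawn a bullet actor or line-trace from the camera, spawning an explosion and pushing physics objects with mass-scaled force.
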(event OnComponentBeginOverlap(CapsuleComponent)
  (params (OverlappedComponent :type Primitive%20Component%20Object%20Reference) (OtherActor :type Actor%20Object%20Reference) (OtherComp :type Primitive%20Component%20Object%20Reference) (OtherBodyIndex :type Integer) (bFromSweep :type Boolean) (SweepResult :type Hit%20Result%20Structure%20%28by%20ref%29))
  ;[1 1 1] Action
)

(event Custom|ChangeGrenadeGun
  (params (bShowGrenade :type Boolean))
  ;[1 1 1] weaponChange
)

(event EventBeginPlay
  ;[1 1 1] crossHair
)

(event Collision|EventActorBeginOverlap
  (params (OtherActor :type Actor%20Object%20Reference)))

(event EventTick
  (params (DeltaSeconds :type Float%20%28single-precision%29))
  ;[1 1 1] moveMent
)

(event Input|ActionEvents|InputActionJump
  (params (Key :type Key%20Structure :default "None"))
  ;[1 1 1] Action
)

(event Input|ActionEvents|InputActionFireBullet
  (params (Key :type Key%20Structure :default "None"))
  ;[1 1 1] Action
)

(event Input|ActionEvents|InputActionGrenadeGun
  (params (Key :type Key%20Structure :default "None"))
  ;[1 1 1] weaponChange
)

(event Input|ActionEvents|InputActionSniperGun
  (params (Key :type Key%20Structure :default "None"))
  ;[1 1 1] weaponChange
)

(event Input|ActionEvents|InputActionSniperZoom
  (params (Key :type Key%20Structure :default "None"))
  ;[1 1 1] Zoom
)

(event Input|ActionEvents|InputActionFireBullet
  (params (Key :type Key%20Structure :default "None")))

(event Input|AxisEvents|InputAxisTurnRight
  (params (AxisValue :type Float%20%28single-precision%29))
  ;[1 1 1] Action
)

(event Input|AxisEvents|InputAxisLookUp
  (params (AxisValue :type Float%20%28single-precision%29))
  ;[1 1 1] Action
)

(fn ConstructionScript)