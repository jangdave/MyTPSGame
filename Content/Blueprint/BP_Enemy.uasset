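; Enemy character that plays a damage reaction montage at the section named by its OnMyDamage event.
; BeginPlay sets the state to IDLE, but Tick is empty.
; A disconnected IDLE/MOVE/ATTACK state machine would target the player pawn, move toward it and switch to a print-only attack within stopping distance.
; An unused node chain builds a random Damage section name.
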(event EventBeginPlay
  (Variables|Default|SetmyState "NewEnumerator0"))

(event Collision|EventActorBeginOverlap
  (params (OtherActor :type Actor%20Object%20Reference)))

(event EventTick
  (params (DeltaSeconds :type Float%20%28single-precision%29)))

(event EventOnMyDamage
  (params (sectionName :type Name :default "None"))
  (Animation|PlayAnimMontage "/Game/Blueprint/EnemyAnimMontage.EnemyAnimMontage" 1.0 sectionName))

(fn ConstructionScript)