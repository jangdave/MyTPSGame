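; Test AI pawn in the Map folder that moves toward pawns it sees.
; PawnSensing's OnSeePawn runs AIMoveTo toward the seen pawn's location at that moment, with a wide acceptance radius.
; The AIPerception update, BeginPlay and Tick events are empty.
; Unconnected AIMoveTo and SimpleMove variants targeting the player remain in the graph as experiments and never run.
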(event OnSeePawn(PawnSensing)
  (params (Pawn :type Pawn%20Object%20Reference))
  (AI|AIMoveTo self (Transformation|GetActorLocation Pawn) 0 5e+02 false))

(event OnTargetPerceptionUpdated(AIPerception)
  (params (Actor :type Actor%20Object%20Reference) (Stimulus :type AI%20Stimulus%20Structure)))

(event EventBeginPlay)

(event Collision|EventActorBeginOverlap
  (params (OtherActor :type Actor%20Object%20Reference)))

(event EventTick
  (params (DeltaSeconds :type Float%20%28single-precision%29)))

(fn ConstructionScript)